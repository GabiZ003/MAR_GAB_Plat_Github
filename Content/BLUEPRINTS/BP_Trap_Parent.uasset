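; BP_Trap_Parent is a base trap Blueprint that damages BP_ThirdPersonCharacter when it overlaps the trap's Box.
; Unless the character is invincible, a hit cuts ENERGIE, refreshes its UI and calls IsInvincible, or calls Isdead if energy is already low.
; BeginPlay calls MoveLoop, an empty event here that child traps can presumably override for movement.
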(event OnComponentBeginOverlap(Box)
  (params (OverlappedComponent :type Primitive%20Component%20Object%20Reference) (OtherActor :type Actor%20Object%20Reference) (OtherComp :type Primitive%20Component%20Object%20Reference) (OtherBodyIndex :type Integer) (bFromSweep :type Boolean) (SweepResult :type Hit%20Result%20Structure%20%28by%20ref%29))
  (bind _asbp_third_person_character (Utilities|Casting|CastToBP_ThirdPersonCharacter OtherActor))
  (if (not (Variables|/Game/ThirdPerson/Blueprints/BP_ThirdPersonCharacter.BP_ThirdPersonCharacter_C|GetInvincible _asbp_third_person_character))
    (if (> (Variables|/Game/ThirdPerson/Blueprints/BP_ThirdPersonCharacter.BP_ThirdPersonCharacter_C|GetENERGIE _asbp_third_person_character) 1.2)
      (if (< (Variables|/Game/ThirdPerson/Blueprints/BP_ThirdPersonCharacter.BP_ThirdPersonCharacter_C|GetENERGIE _asbp_third_person_character) 4.2)
        (Variables|/Game/ThirdPerson/Blueprints/BP_ThirdPersonCharacter.BP_ThirdPersonCharacter_C|SetENERGIE _asbp_third_person_character (Math|Float|Clamp(Float) (- (Variables|/Game/ThirdPerson/Blueprints/BP_ThirdPersonCharacter.BP_ThirdPersonCharacter_C|GetENERGIE _asbp_third_person_character) 3.0) 0.0 5.0))
        (else
          (Variables|/Game/ThirdPerson/Blueprints/BP_ThirdPersonCharacter.BP_ThirdPersonCharacter_C|SetENERGIE _asbp_third_person_character 1.2)))
      (Default|SetEnergiePercent (Variables|/Game/ThirdPerson/Blueprints/BP_ThirdPersonCharacter.BP_ThirdPersonCharacter_C|GetUI _asbp_third_person_character) (/ (Variables|/Game/ThirdPerson/Blueprints/BP_ThirdPersonCharacter.BP_ThirdPersonCharacter_C|GetENERGIE _asbp_third_person_character) 5.0))
      (Default|SetTextEnergie (Variables|/Game/ThirdPerson/Blueprints/BP_ThirdPersonCharacter.BP_ThirdPersonCharacter_C|GetUI _asbp_third_person_character) (Utilities|Text|ToText(Float) (Variables|/Game/ThirdPerson/Blueprints/BP_ThirdPersonCharacter.BP_ThirdPersonCharacter_C|GetENERGIE _asbp_third_person_character) "HalfToEven"))
      (Default|IsInvincible _asbp_third_person_character)
      (else
        (Default|Isdead _asbp_third_person_character)))))

(event Custom|MoveLoop)

(event EventBeginPlay
  (CallFunction|MoveLoop))

(event Collision|EventActorBeginOverlap
  (params (OtherActor :type Actor%20Object%20Reference)))

(event EventTick
  (params (DeltaSeconds :type Float%20%28single-precision%29)))

(fn ConstructionScript)