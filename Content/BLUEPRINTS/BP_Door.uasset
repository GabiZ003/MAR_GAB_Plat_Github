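; BP_Door is a door actor that swings open by rotating around its Z axis.
; When the third-person character enters its Box trigger, the door adds itself to that character's OpenDoors collection; nothing here removes it.
; The Open event stores the current yaw, then plays the Opendoor timeline, adding its AxeZ track to that yaw while keeping location and scale.
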(event OnComponentBeginOverlap(Box)
  (params (OverlappedComponent :type Primitive%20Component%20Object%20Reference) (OtherActor :type Actor%20Object%20Reference) (OtherComp :type Primitive%20Component%20Object%20Reference) (OtherBodyIndex :type Integer) (bFromSweep :type Boolean) (SweepResult :type Hit%20Result%20Structure%20%28by%20ref%29))
  (bind _asbp_third_person_character (Utilities|Casting|CastToBP_ThirdPersonCharacter OtherActor))
  (Utilities|Array|Add (Variables|/Game/ThirdPerson/Blueprints/BP_ThirdPersonCharacter.BP_ThirdPersonCharacter_C|GetOpen_Doors _asbp_third_person_character) self))

(event Custom|Open
  (bind _returnvalue (Transformation|GetActorTransform))
  (Variables|Default|SetRotaZ_initial (.yaw (.rotation (Transformation|GetActorTransform))))
  (bind _axez (Timeline|Opendoor Play)
    (:Update
      (Transformation|SetActorTransform (Math|Transform|MakeTransform (.location _returnvalue) (Math|Rotator|MakeRotator 0.0 0.0 (+ _axez (Variables|Default|GetRotaZ_initial))) (.scale _returnvalue))))))

(event EventBeginPlay)

(event Collision|EventActorBeginOverlap
  (params (OtherActor :type Actor%20Object%20Reference)))

(event EventTick
  (params (DeltaSeconds :type Float%20%28single-precision%29)))

(fn ConstructionScript)